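; BP_Player is the player character, which moves along the world Y axis and fires projectiles through Enhanced Input.
; BeginPlay adds the input mapping context and sets the collider to the mesh's X and Z location.
; Firing spawns a projectile at an offset from the actor.
; A DoOnce reset on release limits fire to one shot per press, and a timer-cleared cooldown flag limits the rate.
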(event `self.ReceiveBeginPlay`
  (bind (_returnvalue_x _returnvalue_y _returnvalue_z) (`KismetMathLibrary.BreakVector` (`SceneComponent.K2_GetComponentLocation` (`self.Mesh`))))
  (bind _returnvalue (pcsubsystem `EnhancedInputLocalPlayerSubsystem` (`GameplayStatics.GetPlayerController` 0)))
  ;[1 0.604 0.614] Adding the Input Mapping Context
  (`/Engine/EditorBlueprintResources/StandardMacros.IsValid` _returnvalue
    (:`Is Valid`
      (`EnhancedInputSubsystemInterface.AddMappingContext` _returnvalue "/Game/Input/IMC_PlayerInput.IMC_PlayerInput" 0 (struct))
      ;[1 1 1] Prevents collider from fully inheriting mesh location
      (`SceneComponent.K2_SetWorldLocation` (`self.Collider`) (`KismetMathLibrary.MakeVector` _returnvalue_x 0.0 _returnvalue_z) false false))))

(event `EnhancedInput|/Game/Input/INP_Movement`
  (params (ActionValue :type "Float (double-precision)") (ElapsedSeconds :type "Float (double-precision)") (TriggeredSeconds :type "Float (double-precision)") (InputAction :type "InputAction Object Reference" :default "/Game/Input/INP_Movement.INP_Movement"))
  ;[0.7312 0.756 1] Movement
  (:`Triggered`
    (`self.AddMovementInput` (`KismetMathLibrary.MakeVector` 0.0 (`self.MovementSpeed`)) ActionValue)))

(event `EnhancedInput|/Game/Input/INP_Fire`
  (params (ActionValue :type Boolean) (ElapsedSeconds :type "Float (double-precision)") (TriggeredSeconds :type "Float (double-precision)") (InputAction :type "InputAction Object Reference" :default "/Game/Input/INP_Fire.INP_Fire"))
  (bind _returnvalue_location (`KismetMathLibrary.BreakTransform` (`self.GetTransform`)))
  ;[1 0.9335 0.5932] Firing
  (:`Triggered`
    (`/Engine/EditorBlueprintResources/StandardMacros.DoOnce` false :!label _label
      (:`Completed`
        (if (not (`self.OnCooldown`))
          (`|SpawnActorFromClass` (`self.Projectile`) (`KismetMathLibrary.Conv_VectorToTransform` (+ _returnvalue_location (`self.ProjectileOffset`))) "Undefined" "MultiplyWithRoot" null null)
          (bind _output_get (set `self.OnCooldown` (not (stale _output_get))))
          (`KismetSystemLibrary.K2_SetTimerDelegate` (delegate `RemoveCooldown`) (`self.ShootSpeed`))))))
  (:`Completed`
    (goto _label :!via `Reset`)))

(event `RemoveCooldown`
  ;[1 0.9335 0.5932] Firing
  (bind _output_get (set `self.OnCooldown` (not (stale _output_get)))))

(fn `UserConstructionScript`)