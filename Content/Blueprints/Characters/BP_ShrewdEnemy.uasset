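; BP_ShrewdEnemy is an enemy Blueprint with a floating health bar widget.
; On BeginPlay it disables the widget's shadow and resets its world scale.
; Each Tick it changes only the widget's pitch to face the player camera, keeping roll and yaw.
; The UpdateHealthBar event casts the widget to WBP_EnemyHealthBar and sets the bar's fill to TempHealth divided by Health.
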(event `self.ReceiveBeginPlay`
  (bind _healthbarwidget (`self.HealthBarWidget`))
  (`PrimitiveComponent.SetCastShadow` _healthbarwidget false)
  (`SceneComponent.SetWorldScale3D` _healthbarwidget (1.0 1.0 1.0)))

(event `self.ReceiveTick`
  (params (DeltaSeconds :type "Float (single-precision)"))
  (bind _healthbarwidget (`self.HealthBarWidget`))
  (bind (_returnvalue_roll _returnvalue_pitch _returnvalue_yaw) (`KismetMathLibrary.BreakRotator` (`SceneComponent.K2_GetComponentRotation` _healthbarwidget)))
  (bind (_returnvalue_roll_2 _returnvalue_pitch_2) (`KismetMathLibrary.BreakRotator` (`KismetMathLibrary.FindLookAtRotation` (`SceneComponent.K2_GetComponentLocation` (`self.HealthBarWidget`)) (`SceneComponent.K2_GetComponentLocation` (`PlayerCameraManager.TransformComponent` (`GameplayStatics.GetPlayerCameraManager` 0))))))
  ;[1 1 1] Health bar rotating in only the Y direction
  (`SceneComponent.K2_SetWorldRotation` _healthbarwidget (`KismetMathLibrary.MakeRotator` _returnvalue_roll _returnvalue_pitch_2 _returnvalue_yaw) false false))

(event `self.UpdateHealthBar`
  ;[1 1 1] Update health bar
  (bind _aswbp_enemy_health_bar (cast `/Game/Blueprints/UI/WBP_EnemyHealthBar` (`WidgetComponent.GetWidget` (`self.HealthBarWidget`))))
  (`ProgressBar.SetPercent` (`/Game/Blueprints/UI/WBP_EnemyHealthBar.HealthBar` _aswbp_enemy_health_bar) (/ (`self.TempHealth`) (`self.Health`))))

(fn `UserConstructionScript`)