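; BP_PlaceableManager controls placement preview feedback, showing whether the current placeable is valid and buyable.
; SetPreviewonSoulChange rechecks IsBuyable, combines it with the stored CanPlace state, then swaps the Preview between correct and wrong materials.
; SetPreviewMaterial responds to a collision flag, updating material and CanPlace only while the item is buyable.
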(event `self.SetPreviewOnSoulChange`
  (bind _returnvalue (`self.IsBuyable`))
  (bind _returnvalue_2 (and _returnvalue (`self.bCanPlace`)))
  (if _returnvalue_2
    (`DDPlaceablePreview.SetMaterial` (`self.Preview`) "/Game/Materials/MI_CorrectPlaceablePreview.MI_CorrectPlaceablePreview")
    (`self.CanPlace` _returnvalue_2)
    (else
      (`DDPlaceablePreview.SetMaterial` (`self.Preview`) "/Game/Materials/MI_WrongPlaceablePreview.MI_WrongPlaceablePreview")
      (`self.CanPlace` _returnvalue_2))))

(event `self.SetPreviewMaterial`
  (params (IsColliding :type Boolean))
  (bind _preview (`self.Preview`))
  (bind _returnvalue (`self.IsBuyable`))
  (if _returnvalue
    (if IsColliding
      (`DDPlaceablePreview.SetMaterial` _preview "/Game/Materials/MI_WrongPlaceablePreview.MI_WrongPlaceablePreview")
      (else
        (`DDPlaceablePreview.SetMaterial` _preview "/Game/Materials/MI_CorrectPlaceablePreview.MI_CorrectPlaceablePreview")))
    (`self.CanPlace` (not IsColliding))))

(fn `UserConstructionScript`)